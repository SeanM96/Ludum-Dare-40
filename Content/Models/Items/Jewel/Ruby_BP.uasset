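; Ruby pickup actor that the player collects as loot, at the cost of movement speed.
; When its Box is overlapped by a ThirdPersonCharacter, it increments that character's TotalLoots and adds AddWeight to TotalWeight.
; It also subtracts the same AddWeight directly from the character's MaxWalkSpeed, with no lower clamp, then destroys itself.
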(event OnComponentBeginOverlap(Box)
  (params (OverlappedComponent :type Primitive%20Component%20Object%20Reference) (OtherActor :type Actor%20Object%20Reference) (OtherComp :type Primitive%20Component%20Object%20Reference) (OtherBodyIndex :type Integer) (bFromSweep :type Boolean) (SweepResult :type Hit%20Result%20Structure%20%28by%20ref%29))
  (bind _addweight (Variables|Default|GetaddWeight))
  (bind _asthird_person_character (Utilities|Casting|CastToThirdPersonCharacter OtherActor))
  (Variables|/Game/Map/Blueprints/ThirdPersonCharacter.ThirdPersonCharacter_C|SetTotalLoots _asthird_person_character (+ (Variables|/Game/Map/Blueprints/ThirdPersonCharacter.ThirdPersonCharacter_C|GetTotalLoots _asthird_person_character) 1))
  (Variables|/Game/Map/Blueprints/ThirdPersonCharacter.ThirdPersonCharacter_C|SettotalWeight _asthird_person_character (+ (Variables|/Game/Map/Blueprints/ThirdPersonCharacter.ThirdPersonCharacter_C|GettotalWeight _asthird_person_character) _addweight))
  (Variables|/Script/Engine.CharacterMovementComponent|SetMaxWalkSpeed (Variables|/Script/Engine.Character|GetCharacterMovement _asthird_person_character) (- (Variables|/Script/Engine.CharacterMovementComponent|GetMaxWalkSpeed (Variables|/Script/Engine.Character|GetCharacterMovement _asthird_person_character)) (Math|Conversions|ToFloat(Integer) _addweight)))
  (Actor|DestroyActor self))

(fn ConstructionScript)